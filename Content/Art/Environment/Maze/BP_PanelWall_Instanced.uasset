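; Maze panel wall actor that fills a spline with randomly varied instanced static meshes at construction time.
; The construction script assigns NewMeshI to one randomly chosen component of ten, then derives segment spacing from that mesh's X bounds and the actor's X scale.
; It steps along the spline at that spacing, adding each location-only local-space instance, without spline rotation, to a randomly picked component.
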(event EventBeginPlay)

(event Collision|EventActorBeginOverlap
  (params (OtherActor :type Actor%20Object%20Reference)))

(event EventTick
  (params (DeltaSeconds :type Float%20%28single-precision%29)))

(fn ConstructionScript
  (bind _returnvalue (Math|Random|RandomIntegerinRange 0 9))
  (bind _new_mesh_i (Variables|Default|GetNew%20Mesh_I))
  (bind _instancedstaticmesh_1 (Variables|Default|GetInstancedStaticMesh_1))
  (bind _instancedstaticmesh_2 (Variables|Default|GetInstancedStaticMesh_2))
  (bind _instancedstaticmesh_3 (Variables|Default|GetInstancedStaticMesh_3))
  (bind _instancedstaticmesh_4 (Variables|Default|GetInstancedStaticMesh_4))
  (bind _instancedstaticmesh_5 (Variables|Default|GetInstancedStaticMesh_5))
  (bind _instancedstaticmesh_6 (Variables|Default|GetInstancedStaticMesh_6))
  (bind _instancedstaticmesh_8 (Variables|Default|GetInstancedStaticMesh_8))
  (bind _instancedstaticmesh_9 (Variables|Default|GetInstancedStaticMesh_9))
  (bind _instancedstaticmesh_10 (Variables|Default|GetInstancedStaticMesh_10))
  (bind _instancedstaticmesh_7 (Variables|Default|GetInstancedStaticMesh_7))
  (bind _returnvalue_2 (StaticMesh|GetBoundingBox _new_mesh_i))
  (bind _returnvalue_3 (Utilities|Select :Index _returnvalue :Option%200 _instancedstaticmesh_1 :Option%201 _instancedstaticmesh_2 :Option%202 _instancedstaticmesh_3 :Option%203 _instancedstaticmesh_4 :Option%204 _instancedstaticmesh_5 :Option%205 _instancedstaticmesh_6 :Option%206 _instancedstaticmesh_7 :Option%207 _instancedstaticmesh_8 :Option%208 _instancedstaticmesh_9 :Option%209 _instancedstaticmesh_10))
  (bind (_min _max) (Utilities|Struct|BreakBox _returnvalue_2))
  (Components|StaticMesh|SetStaticMesh _returnvalue_3 (Variables|Default|GetNew%20Mesh_I))
  (Variables|Default|SetSectionLenght%20Coef (- (.x _max) (.x _min)))
  (Variables|Default|SetLenght (* (.x (Transformation|GetActorScale3D)) (Variables|Default|GetSectionLenght%20Coef)))
  (for _index (range 0 (- (Math|Float|Truncate (/ (Spline|GetSplineLength (Variables|Default|GetSpline)) (Variables|Default|GetLenght))) 1))
    (Variables|Default|SetIndex _index)
    (Components|InstancedStaticMesh|AddInstance _returnvalue_3 (Math|Conversions|ToTransform(Vector) (Spline|GetLocationatDistanceAlongSpline (Variables|Default|GetSpline) (* (Variables|Default|GetIndex) (Variables|Default|GetLenght)) "Local")) false)))