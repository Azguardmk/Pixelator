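; Spline-driven decoration actor, named as a road fence, that builds a chain of deformed mesh segments along its spline in the construction script.
; The spline length is split into whole segments near Length, stretched evenly to fill it.
; Each spline mesh follows local positions and clamped tangents, with its start pulled back by Offset.
; Each pass also adds an instanced mesh component and assigns SplineMesh through the ISM variable, but adds no instances.
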(event Collision|EventActorBeginOverlap
  (params (OtherActor :type Actor%20Object%20Reference)))

(event EventTick
  (params (DeltaSeconds :type Float%20%28single-precision%29)))

(fn ConstructionScript
  (bind _length (Variables|Default|GetLength))
  (bind _spline (Variables|Default|GetSpline))
  (bind _spline_2 (Variables|Default|GetSpline))
  (bind _returnvalue (Spline|GetSplineLength _spline))
  (bind _returnvalue_2 (/ _returnvalue _length))
  (bind _returnvalue_3 (Math|Float|Floor _returnvalue_2))
  (Variables|Default|SetNewLength (/ _returnvalue (Math|Conversions|ToFloat(Integer) _returnvalue_3)))
  (for _index (range 0 (- _returnvalue_3 1))
    (bind _returnvalue_4 (AddComponent|AddSplineMeshComponent false))
    (Components|StaticMesh|SetStaticMesh (Variables|Default|GetISM) (Variables|Default|GetSplineMesh))
    (bind _returnvalue_5 (AddComponent|AddInstancedStaticMeshComponent false))
    (Variables|Default|SetISM _returnvalue_5)
    (SplineMesh|SetStartandEnd _returnvalue_4 (Spline|GetLocationatDistanceAlongSpline _spline_2 (- (* _index (Variables|Default|GetNewLength)) (Variables|Default|GetOffset)) "Local") (Math|Vector|ClampVectorSize (Spline|GetTangentatDistanceAlongSpline _spline_2 (- (* _index (Variables|Default|GetNewLength)) (Variables|Default|GetOffset)) "Local") 0.0 (Variables|Default|GetNewLength)) (Spline|GetLocationatDistanceAlongSpline _spline_2 (* (+ _index 1) (Variables|Default|GetNewLength)) "Local") (Math|Vector|ClampVectorSize (Spline|GetTangentatDistanceAlongSpline _spline_2 (* (+ _index 1) (Variables|Default|GetNewLength)) "Local") 0.0 (Variables|Default|GetNewLength)) true :!class /Script/Engine.SplineMeshComponent)))