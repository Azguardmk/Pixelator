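; Decorative suspension bridge actor that builds itself along a spline from randomly chosen mesh pieces.
; The construction script divides the spline by a segment length, stretching the spacing so whole pieces fill it exactly.
; Each segment adds a mesh component with one of three random bridge meshes, shaped by spline start/end points and clamped tangents.
; An offset pulls each start back along the spline; randomness is unseeded, so reconstruction reshuffles pieces.
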(event EventBeginPlay)

(event Collision|EventActorBeginOverlap
  (params (OtherActor :type Actor%20Object%20Reference)))

(event EventTick
  (params (DeltaSeconds :type Float%20%28single-precision%29)))

(fn ConstructionScript
  (bind _spline (Variables|Default|GetSpline))
  (bind _spline_2 (Variables|Default|GetSpline))
  (bind _lenght (Variables|Default|GetLenght))
  (bind _returnvalue (Spline|GetSplineLength _spline))
  (bind _returnvalue_2 (/ _returnvalue _lenght))
  (bind _returnvalue_3 (Math|Float|Floor _returnvalue_2))
  ;[1 1 1] Spline_Lenght Adjustment
  (Variables|Default|SetNewLength (/ _returnvalue (Math|Conversions|ToFloat(Integer) _returnvalue_3)))
  (for _index (range 0 (- _returnvalue_3 1))
    (bind _returnvalue_4 (AddComponent|AddInstancedStaticMeshComponent false))
    ;[1 0.9989 0.3979] Add Random Mesh
    (Components|StaticMesh|SetStaticMesh _returnvalue_4 (Utilities|Array|Get(acopy) (Variables|Default|GetBridgeMesh) (Math|Random|RandomIntegerinRange 0 2)))
    (SplineMesh|SetForwardAxis 0 "X" true)
    (SplineMesh|SetStartandEnd 0 (Spline|GetLocationatDistanceAlongSpline _spline_2 (- (* _index (Variables|Default|GetNewLength)) (Variables|Default|GetOffset)) "Local") (Math|Vector|ClampVectorSize (Spline|GetTangentatDistanceAlongSpline _spline_2 (- (* _index (Variables|Default|GetNewLength)) (Variables|Default|GetOffset)) "Local") 0.0 (Variables|Default|GetNewLength)) (Spline|GetLocationatDistanceAlongSpline _spline_2 (* (+ _index 1) (Variables|Default|GetNewLength)) "Local") (Math|Vector|ClampVectorSize (Spline|GetTangentatDistanceAlongSpline _spline_2 (* (+ _index 1) (Variables|Default|GetNewLength)) "Local") 0.0 (Variables|Default|GetNewLength)) true :!class /Script/Engine.SplineMeshComponent)))