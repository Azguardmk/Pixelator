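; BP_WallPanelsMaze is a construction-script actor that lines a spline with instanced wall panels, by its name for building mazes.
; It assigns one random InputMesh entry to ISM1, then derives spacing from X bounds plus Offset, using separate random picks.
; It adds unrotated instances at that spacing along the spline length.
; An unconnected per-instance randomisation branch and an unused added ISM component remain; runtime events are empty.
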(event EventBeginPlay)

(event Collision|EventActorBeginOverlap
  (params (OtherActor :type Actor%20Object%20Reference)))

(event EventTick
  (params (DeltaSeconds :type Float%20%28single-precision%29)))

(fn ConstructionScript
  (bind _returnvalue (Math|Random|RandomIntegerinRange 0 9))
  (bind _inputmesh (Variables|Default|GetInputMesh))
  (bind _output (Utilities|Array|Get(acopy) _inputmesh _returnvalue))
  (bind _returnvalue_2 (StaticMesh|GetBoundingBox _output))
  (bind (_min _max) (Utilities|Struct|BreakBox _returnvalue_2))
  (Components|StaticMesh|SetStaticMesh (Variables|Default|GetISM_1) _output)
  (AddComponent|AddInstancedStaticMeshComponent false)
  (bind _output_get (Variables|Default|SetSpacing (+ (.X (Math|Vector|BreakVector (- _max _min))) (Variables|Default|GetOffset)))) ; NewSize of the mesh+offset (Spacing = 100... as an exsample)
  (bind _output_get_2 (Variables|Default|SetNumberOfInstances (Math|Float|Floor (/ (Spline|GetSplineLength (Variables|Default|GetSpline)) _output_get))))
  (for _index (range 0 _output_get_2) ; Repeat as many times, as there are Number of instances
    (Components|InstancedStaticMesh|AddInstance (Variables|Default|GetISM_1) (Math|Transform|MakeTransform (Spline|GetLocationatDistanceAlongSpline (Variables|Default|GetSpline) (* _index (Variables|Default|GetSpacing)) "Local")) false) ; Adds this mesh to the point
  ))